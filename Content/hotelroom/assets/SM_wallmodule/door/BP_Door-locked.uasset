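; BP_Door-locked is a locked hotel room door that rattles when the player presses F nearby instead of opening.
; Overlapping Box1 enables input on the actor and leaving it disables input.
; The F press plays an ActorSequence forward and in reverse twice with short delays, while the AnimationPast flag blocks retriggering until the rattle finishes.
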(event `Key|F`
  (params (Key :type "Key Structure"))
  (bind _sequenceplayer (`ActorSequenceComponent.SequencePlayer` (`self.ActorSequence`)))
  (:`Pressed`
    (if (`self.animation past? `)
      (set `self.animation past? ` false)
      (`MovieSceneSequencePlayer.Play` _sequenceplayer)
      (`KismetSystemLibrary.Delay` 0.2)
      (`MovieSceneSequencePlayer.PlayReverse` _sequenceplayer)
      (`KismetSystemLibrary.Delay` 0.2)
      (`MovieSceneSequencePlayer.Play` _sequenceplayer)
      (`KismetSystemLibrary.Delay` 0.2)
      (`MovieSceneSequencePlayer.PlayReverse` _sequenceplayer)
      (`KismetSystemLibrary.Delay` 0.2)
      (set `self.animation past? ` true))))

(event `self.Box1.OnComponentBeginOverlap`
  (params (OverlappedComponent :type "PrimitiveComponent Object Reference") (OtherActor :type "Actor Object Reference") (OtherComp :type "PrimitiveComponent Object Reference") (OtherBodyIndex :type Integer) (bFromSweep :type Boolean) (SweepResult :type "HitResult Structure (by ref)"))
  ;[1 1 1] Comment
  (`self.EnableInput` (`GameplayStatics.GetPlayerController` 0)))

(event `self.Box1.OnComponentEndOverlap`
  (params (OverlappedComponent :type "PrimitiveComponent Object Reference") (OtherActor :type "Actor Object Reference") (OtherComp :type "PrimitiveComponent Object Reference") (OtherBodyIndex :type Integer))
  ;[1 1 1] Comment
  (`self.DisableInput` (`GameplayStatics.GetPlayerController` 0)))

(fn `UserConstructionScript`)