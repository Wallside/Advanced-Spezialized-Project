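; Elevator actor for the hotel room assets, animated by two Actor Sequence components.
; The first character overlap with Box1 plays sequence one.
; Box2 enables player input only during overlap, without filtering actors, so F can trigger the ride.
; The first F press reverses sequence one, then plays sequence two forward, backward and forward on fixed delays, with neither DoOnce ever reset.
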(event `self.Box1.OnComponentBeginOverlap`
  (params (OverlappedComponent :type "PrimitiveComponent Object Reference") (OtherActor :type "Actor Object Reference") (OtherComp :type "PrimitiveComponent Object Reference") (OtherBodyIndex :type Integer) (bFromSweep :type Boolean) (SweepResult :type "HitResult Structure (by ref)"))
  ;[1 1 1] Comment
  (cast `/Game/FirstPersonBP/Blueprints/FirstPersonCharacter` OtherActor)
  (`/Engine/EditorBlueprintResources/StandardMacros.DoOnce` false
    (:`Completed`
      (`MovieSceneSequencePlayer.Play` (`ActorSequenceComponent.SequencePlayer` (`self.ActorSequence1`))))))

(event `Key|F`
  (params (Key :type "Key Structure"))
  (bind _sequenceplayer (`ActorSequenceComponent.SequencePlayer` (`self.ActorSequence2`)))
  (:`Pressed`
    (`/Engine/EditorBlueprintResources/StandardMacros.DoOnce` false
      (:`Completed`
        (`MovieSceneSequencePlayer.PlayReverse` (`ActorSequenceComponent.SequencePlayer` (`self.ActorSequence1`)))
        (`KismetSystemLibrary.Delay` 5.0)
        (`MovieSceneSequencePlayer.Play` _sequenceplayer)
        (`KismetSystemLibrary.Delay` 7.0)
        (`MovieSceneSequencePlayer.PlayReverse` _sequenceplayer)
        (`KismetSystemLibrary.Delay` 7.0)
        (`MovieSceneSequencePlayer.Play` _sequenceplayer)))))

(event `self.Box2.OnComponentBeginOverlap`
  (params (OverlappedComponent :type "PrimitiveComponent Object Reference") (OtherActor :type "Actor Object Reference") (OtherComp :type "PrimitiveComponent Object Reference") (OtherBodyIndex :type Integer) (bFromSweep :type Boolean) (SweepResult :type "HitResult Structure (by ref)"))
  ;[1 1 1] Comment
  (`self.EnableInput` (`GameplayStatics.GetPlayerController` 0)))

(event `self.Box2.OnComponentEndOverlap`
  (params (OverlappedComponent :type "PrimitiveComponent Object Reference") (OtherActor :type "Actor Object Reference") (OtherComp :type "PrimitiveComponent Object Reference") (OtherBodyIndex :type Integer))
  ;[1 1 1] Comment
  (`self.DisableInput` (`GameplayStatics.GetPlayerController` 0)))

(fn `UserConstructionScript`)