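; Hotel room dresser Blueprint with three interactive parts that the player toggles with the F key.
; Trigger boxes enable player input and set a per-part flag on overlap, then disable input and clear it on exit.
; For whichever flag is set, F drives a FlipFlop that alternately plays that part's Actor Sequence forward and in reverse.
; The third part shares its logic between two trigger boxes.
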(event `self.Box1.OnComponentBeginOverlap`
  (params (OverlappedComponent :type "PrimitiveComponent Object Reference") (OtherActor :type "Actor Object Reference") (OtherComp :type "PrimitiveComponent Object Reference") (OtherBodyIndex :type Integer) (bFromSweep :type Boolean) (SweepResult :type "HitResult Structure (by ref)"))
  ;[1 1 1] Comment
  (`self.EnableInput` (`GameplayStatics.GetPlayerController` 0))
  (set `self.in box1?` true))

(event `Key|F`
  (params (Key :type "Key Structure"))
  (bind _sequenceplayer (`ActorSequenceComponent.SequencePlayer` (`self.ActorSequence1`)))
  ;[1 1 1] Comment
  (:`Pressed`
    (if (`self.in box1?`)
      (`/Engine/EditorBlueprintResources/StandardMacros.FlipFlop`
        (:`A`
          (`MovieSceneSequencePlayer.Play` _sequenceplayer))
        (:`B`
          (`MovieSceneSequencePlayer.PlayReverse` _sequenceplayer))))))

(event `self.Box1.OnComponentEndOverlap`
  (params (OverlappedComponent :type "PrimitiveComponent Object Reference") (OtherActor :type "Actor Object Reference") (OtherComp :type "PrimitiveComponent Object Reference") (OtherBodyIndex :type Integer))
  ;[1 1 1] Comment
  (`self.DisableInput` (`GameplayStatics.GetPlayerController` 0))
  (set `self.in box1?` false))

(event `self.Box2.OnComponentBeginOverlap`
  (params (OverlappedComponent :type "PrimitiveComponent Object Reference") (OtherActor :type "Actor Object Reference") (OtherComp :type "PrimitiveComponent Object Reference") (OtherBodyIndex :type Integer) (bFromSweep :type Boolean) (SweepResult :type "HitResult Structure (by ref)"))
  ;[1 1 1] Comment
  (`self.EnableInput` (`GameplayStatics.GetPlayerController` 0))
  (set `self.in box2?` true))

(event `Key|F`
  (params (Key :type "Key Structure"))
  (bind _sequenceplayer (`ActorSequenceComponent.SequencePlayer` (`self.ActorSequence2`)))
  ;[1 1 1] Comment
  (:`Pressed`
    (if (`self.in box2?`)
      (`/Engine/EditorBlueprintResources/StandardMacros.FlipFlop`
        (:`A`
          (`MovieSceneSequencePlayer.Play` _sequenceplayer))
        (:`B`
          (`MovieSceneSequencePlayer.PlayReverse` _sequenceplayer))))))

(event `self.Box2.OnComponentEndOverlap`
  (params (OverlappedComponent :type "PrimitiveComponent Object Reference") (OtherActor :type "Actor Object Reference") (OtherComp :type "PrimitiveComponent Object Reference") (OtherBodyIndex :type Integer))
  ;[1 1 1] Comment
  (`self.DisableInput` (`GameplayStatics.GetPlayerController` 0))
  (set `self.in box2?` false))

(event `Key|F`
  (params (Key :type "Key Structure"))
  (bind _sequenceplayer (`ActorSequenceComponent.SequencePlayer` (`self.ActorSequence3`)))
  ;[1 1 1] Comment
  (:`Pressed`
    (if (`self.in box3?`)
      (`/Engine/EditorBlueprintResources/StandardMacros.FlipFlop`
        (:`A`
          (`MovieSceneSequencePlayer.Play` _sequenceplayer))
        (:`B`
          (`MovieSceneSequencePlayer.PlayReverse` _sequenceplayer))))))

(event `self.Box3.1.OnComponentBeginOverlap`
  (params (OverlappedComponent :type "PrimitiveComponent Object Reference") (OtherActor :type "Actor Object Reference") (OtherComp :type "PrimitiveComponent Object Reference") (OtherBodyIndex :type Integer) (bFromSweep :type Boolean) (SweepResult :type "HitResult Structure (by ref)"))
  ;[1 1 1] Comment
  (`self.EnableInput` (`GameplayStatics.GetPlayerController` 0) :!label _label)
  (set `self.in box3?` true))

(event `self.Box3.2.OnComponentBeginOverlap`
  (params (OverlappedComponent :type "PrimitiveComponent Object Reference") (OtherActor :type "Actor Object Reference") (OtherComp :type "PrimitiveComponent Object Reference") (OtherBodyIndex :type Integer) (bFromSweep :type Boolean) (SweepResult :type "HitResult Structure (by ref)"))
  (goto _label))

(event `self.Box3.1.OnComponentEndOverlap`
  (params (OverlappedComponent :type "PrimitiveComponent Object Reference") (OtherActor :type "Actor Object Reference") (OtherComp :type "PrimitiveComponent Object Reference") (OtherBodyIndex :type Integer))
  ;[1 1 1] Comment
  (`self.DisableInput` (`GameplayStatics.GetPlayerController` 0) :!label _label_2)
  (set `self.in box3?` false))

(event `self.Box3.2.OnComponentEndOverlap`
  (params (OverlappedComponent :type "PrimitiveComponent Object Reference") (OtherActor :type "Actor Object Reference") (OtherComp :type "PrimitiveComponent Object Reference") (OtherBodyIndex :type Integer))
  (goto _label_2))

(fn `UserConstructionScript`)